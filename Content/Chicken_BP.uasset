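; Chicken actor that the player steers, and that gets squashed when a car or truck hits it.
; Overlapping BlueCar_BP or truck_BP turns off player control and sets a new actor transform scaled wide in X and Y.
; The MoveLeft press, gated by the control and Jumping flags, sets a fixed relative rotation and location.
; Jumping is never cleared after that press, so the move fires only once.
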(event EventBeginPlay
  (Variables|Default|Setpcontrol true)
  (Variables|Default|Setjumping false))

(event Collision|EventActorBeginOverlap
  (params (OtherActor :type Actor%20Object%20Reference))
  (Utilities|Casting|CastToBlueCar_BP OtherActor
    (:then
      _)
    (:CastFailed
      (Utilities|Casting|CastTotruck_BP OtherActor)))
  (Variables|Default|Setpcontrol false)
  (Transformation|SetActorTransform (Math|Transform|MakeTransform "0, 0, 0" "0, 0, 0" "10.000000,10.000000,1.000000")))

(event EventTick
  (params (DeltaSeconds :type Float%20%28single-precision%29)))

(event Input|ActionEvents|InputActionMoveLeft
  (params (Key :type Key%20Structure))
  (:Pressed
    (if (and (Variables|Default|Getpcontrol) (not (Variables|Default|Getjumping)))
      (Variables|Default|Setjumping true)
      (Transformation|SetActorRelativeRotation "0,-90.000000, 0")
      (Transformation|SetActorRelativeLocation "-25.000000, 0, 0"))))

(fn ConstructionScript)