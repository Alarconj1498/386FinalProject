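; Water actor that sets up a log lane by spawning a log spawner and a deleter around itself.
; On its first Tick, guarded by a Setup flag, it places a LogSpawnerBlueprint on the positive X side and a Deleter_Blueprint on the negative X side, both offset from its own location.
; BeginPlay, overlap and construction script are empty, so this one-time spawn is its only logic.
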(event EventBeginPlay)

(event Collision|EventActorBeginOverlap
  (params (OtherActor :type Actor%20Object%20Reference)))

(event EventTick
  (params (DeltaSeconds :type Float%20%28single-precision%29))
  (bind _returnvalue (Transformation|GetActorLocation))
  (bind _returnvalue_2 (Transformation|GetActorLocation))
  (if (not (Variables|Default|Getsetup))
    (Game|SpawnActorfromClass "/Game/Deleter_Blueprint.Deleter_Blueprint_C" (Math|Transform|MakeTransform (Math|Vector|MakeVector (+ (.x _returnvalue) -4e+01) (+ (.y _returnvalue) -25.0) (+ (.z _returnvalue) 3e+01)) "0, 0, 0" "1.000000,1.000000,1.000000") "Undefined" 0 0)
    (Game|SpawnActorfromClass "/Game/LogSpawnerBlueprint.LogSpawnerBlueprint_C" (Math|Transform|MakeTransform (Math|Vector|MakeVector (+ (.x _returnvalue_2) 2.5e+02) (+ (.y _returnvalue_2) -25.0) (+ (.z _returnvalue_2) 3e+01)) "0, 0, 0" "1.000000,1.000000,1.000000") "Undefined" 0 0)
    (Variables|Default|Setsetup true)))

(fn ConstructionScript)