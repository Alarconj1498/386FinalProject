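; Road lane actor that sets up one-way vehicle traffic when it enters the level.
; On its first Tick, guarded by a Setup flag, it spawns a Deleter at one end and randomly a car spawner (about 70%) or truck spawner toward the other.
; Dir picks which end gets which; non-negative roads also set the spawner's Dir to 1, while negative roads leave its default.
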(event EventBeginPlay)

(event Collision|EventActorBeginOverlap
  (params (OtherActor :type Actor%20Object%20Reference)))

(event EventTick
  (params (DeltaSeconds :type Float%20%28single-precision%29))
  (bind _returnvalue (Transformation|GetActorLocation))
  (bind _returnvalue_2 (Transformation|GetActorLocation))
  (bind _returnvalue_3 (Transformation|GetActorLocation))
  (bind _returnvalue_4 (Transformation|GetActorLocation))
  (bind _returnvalue_5 (+ (.y _returnvalue_2) -25.0))
  (bind _returnvalue_6 (+ (.z _returnvalue_2) 3e+01))
  (bind _returnvalue_7 (+ (.x _returnvalue_4) 2.5e+02))
  (bind _returnvalue_8 (+ (.y _returnvalue_4) -25.0))
  (bind _returnvalue_9 (+ (.z _returnvalue_4) 3e+01))
  (bind _returnvalue_10 (+ (.x _returnvalue_2) 0.0))
  (if (not (Variables|Default|Getsetup))
    (if (< (Variables|Default|Getdir) 0)
      (Game|SpawnActorfromClass "/Game/Deleter_Blueprint.Deleter_Blueprint_C" (Math|Transform|MakeTransform (Math|Vector|MakeVector (+ (.x _returnvalue_3) -4e+01) (+ (.y _returnvalue_3) -25.0) (+ (.z _returnvalue_3) 3e+01)) "0, 0, 0" "1.000000,1.000000,1.000000") "Undefined" 0 0)
      (if (< (Math|Random|RandomFloat) 0.7)
        (Game|SpawnActorfromClass "/Game/CarSpawnerBlueprint.CarSpawnerBlueprint_C" (Math|Transform|MakeTransform (Math|Vector|MakeVector _returnvalue_7 _returnvalue_8 _returnvalue_9) "0, 0, 0" "1.000000,1.000000,1.000000") "Undefined" 0 0)
        (else
          (Game|SpawnActorfromClass "/Game/TruckSpawnerBlueprint.TruckSpawnerBlueprint_C" (Math|Transform|MakeTransform (Math|Vector|MakeVector _returnvalue_7 _returnvalue_8 _returnvalue_9) "0, 0, 0" "1.000000,1.000000,1.000000") "Undefined" 0 0)))
      (Variables|Default|Setsetup true)
      (else
        (Game|SpawnActorfromClass "/Game/Deleter_Blueprint.Deleter_Blueprint_C" (Math|Transform|MakeTransform (Math|Vector|MakeVector (+ (.x _returnvalue) 2.9e+02) (+ (.y _returnvalue) -25.0) (+ (.z _returnvalue) 3e+01)) "0, 0, 0" "1.000000,1.000000,1.000000") "Undefined" 0 0)
        (if (< (Math|Random|RandomFloat) 0.7)
          (bind _returnvalue_11 (Game|SpawnActorfromClass "/Game/CarSpawnerBlueprint.CarSpawnerBlueprint_C" (Math|Transform|MakeTransform (Math|Vector|MakeVector _returnvalue_10 _returnvalue_5 _returnvalue_6) "0, 0, 0" "1.000000,1.000000,1.000000") "Undefined" 0 0))
          (Variables|Default|Setsetup true)
          (Variables|/Game/CarSpawnerBlueprint.CarSpawnerBlueprint_C|Setdir _returnvalue_11 1)
          (else
            (bind _returnvalue_12 (Game|SpawnActorfromClass "/Game/TruckSpawnerBlueprint.TruckSpawnerBlueprint_C" (Math|Transform|MakeTransform (Math|Vector|MakeVector _returnvalue_10 _returnvalue_5 _returnvalue_6) "0, 0, 0" "1.000000,1.000000,1.000000") "Undefined" 0 0))
            (Variables|Default|Setsetup true)
            (Variables|/Game/TruckSpawnerBlueprint.TruckSpawnerBlueprint_C|Setdir _returnvalue_12 1)))))))

(fn ConstructionScript)